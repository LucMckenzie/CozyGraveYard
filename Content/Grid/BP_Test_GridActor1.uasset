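; Test grid actor that lays out a GridX by GridY field of tiles as instanced static meshes.
; The construction script adds one instance per cell, spaced by TileSize and offset by half the grid dimensions around the origin.
; LocationCalucalteSnap is meant as a snap-to-location helper, but only checks the mesh component itself, so it returns that component's world location rather than the nearest tile.
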(fn `LocationCalucalteSnap`
  (params (in :type "Vector Structure"))
  (returns (out :type "Vector Structure"))
  (locals (Closests :type "Vector Structure") (Distance :type "Float (double-precision)"))
  (bind _returnvalue (`SceneComponent.K2_GetComponentLocation` (`self.InstancedStaticMesh`)))
  ;[1 1 1] Snap to Location
  (bind _output_get (set `local.Closests` _returnvalue))
  (set `local.Distance` (`KismetMathLibrary.Vector_Distance` in _returnvalue))
  (for _array_element (`|MakeArray` (`self.InstancedStaticMesh`))
    (bind _returnvalue_2 (`SceneComponent.K2_GetComponentLocation` _array_element))
    (bind _returnvalue_3 (`KismetMathLibrary.Vector_Distance` _returnvalue_2 _output_get))
    (if (< _returnvalue_3 (`local.Distance`))
      (set `local.Closests` _returnvalue_2)
      (set `local.Distance` _returnvalue_3)))
  (return (`local.Closests`)))

(fn `UserConstructionScript`
  (bind _gridx (`self.GridX`))
  (bind _gridy (`self.GridY`))
  (bind _tilesize (`self.TileSize`))
  (for _index (range _gridx)
    (for _index_2 (range _gridy)
      (`InstancedStaticMeshComponent.AddInstance` (`self.InstancedStaticMesh`) (`KismetMathLibrary.MakeTransform` (`KismetMathLibrary.MakeVector` (`KismetMathLibrary.Conv_IntToDouble` (* (- (/ _gridy 2) _index_2) _tilesize)) (`KismetMathLibrary.Conv_IntToDouble` (* (- (/ _gridx 2) _index) _tilesize))))))))