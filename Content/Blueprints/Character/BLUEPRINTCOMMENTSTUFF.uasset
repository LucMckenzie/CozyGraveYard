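; Character Blueprint with unconnected draft logic for eight-direction Paper2D sprite animation, with no event driving it.
; Vertical and horizontal checks, fed placeholder zeros, set heading flags that resolve into a clockwise Direction index from north and a Walking flag.
; Walking and Direction then select PlayerSprite's flipbook.
; Flipbook mapping is unfinished: west-side walking reuses east-side flipbooks, several standing cases use walk flipbooks, and StandNW sits on a stray node.
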(fn `UserConstructionScript`)