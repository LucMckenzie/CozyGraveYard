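; Player character for a grave-tending game, handling movement, item carrying, UI and day progression.
; Overlapped tagged items attach to a socket and register in the inventory; a held garbage bag collects up to three weeds, emptied at bins.
; Q opens the pause menu or, at a bed, saves progress through the GameMode and reloads the level.
; Also feeds memorial items into their widget and locks movement at grave-camera triggers while carrying a memory box.
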(event `InputAxis|MoveForward/Backward`
  (params (AxisValue :type "Float (single-precision)"))
  ;[1 1 1] Movment
  (`self.AddMovementInput` (`KismetMathLibrary.GetForwardVector` (`KismetMathLibrary.MakeRotator` 0.0 0.0 (.yaw (`self.GetControlRotation`)))) AxisValue))

(event `InputAxis|MoveRight/Left`
  (params (AxisValue :type "Float (single-precision)"))
  ;[1 1 1] Movment
  (`self.AddMovementInput` (`KismetMathLibrary.GetRightVector` (`KismetMathLibrary.MakeRotator` 0.0 0.0 (.yaw (`self.GetControlRotation`)))) AxisValue))

(event `InputAction|Pick Up (E)`
  (params (Key :type "Key Structure"))
  (bind _helditem (`self.HeldItem`))
  ;[1 1 1] Pick Up Item
  (:`Pressed`
    (if (`self.Is Holding`) :!label _label
      (`|ExecutionSequence`
        (:`then_0`
          (if (`self.IsOverlappingActor` self (stale `Pick Up Weeds` _array_element))
            (if (`self.Is Holding Garbage`)
              (`self.Pick Up Weeds`)
              (else
                ;[1 1 1] DropItem (Key Version)
                (bind _returnvalue (`GameplayStatics.GetActorOfClass` (`self.Garbage Bin`) :!label _label_2))
                ;;[1 1 1] Stops Garbage bag frombeing dropped when weeds are cleared
                (if (`self.HoldingWeed`)
                  (if (not (`self.IsOverlappingActor` self _returnvalue))
                    (if (`self.Is Holding`) :!label _label_3
                      (bind (_outhit _returnvalue_2) (`KismetSystemLibrary.LineTraceSingle` (`self.K2_GetActorLocation`) (- (`self.K2_GetActorLocation`) (500.0 500.0 500.0)) "TraceTypeQuery1"))
                      (if _returnvalue_2
                        (`self.K2_DetachFromActor` _helditem "KeepWorld" "KeepWorld" "KeepWorld")
                        (`self.K2_SetActorTransform` _helditem (`KismetMathLibrary.MakeTransform` (`.Location` (`GameplayStatics.BreakHitResult` _outhit))) false false)
                        (`/Game/Menus_And_Widgets/W_Inventory.RemoveItemKey` (`self.Inventory`))
                        (set `self.Is Holding` false)
                        (set `self.Is Holding Garbage` false)
                        (set `self.IsHoldingMemoryBox` false))))
                  (else
                    (goto _label_3)))))
            (else
              (goto _label_2))))
        (:`then_1`
          (goto _label_4 :!via `Reset`)))
      (else
        (for _array_element (`self.GetOverlappingActors` "/Game/Blueprints/Items/BP_ItemTest_P.BP_ItemTest_P_C")
          (`/Engine/EditorBlueprintResources/StandardMacros.DoOnce` false :!label _label_4
            (:`Completed`
              (if (`self.ActorHasTag` _array_element "PickUpAble")
                (if (`self.ActorHasTag` _array_element "Garbage")
                  (set `self.Is Holding Garbage` true)
                  (`KismetSystemLibrary.PrintString` "Garbage")
                  (`self.Create Garbage Bag Array`)
                  (else
                    (`KismetSystemLibrary.PrintString` "No Garbage")
                    (if (`self.ActorHasTag` _array_element "MemoryBox")
                      (`KismetSystemLibrary.PrintString` "Holding Box")
                      (set `self.IsHoldingMemoryBox` true)
                      (else
                        (`KismetSystemLibrary.PrintString` "No Box")))))
                (bind _output_get (set `self.HeldItem` _array_element))
                (`self.K2_AttachToComponent` _output_get (`self.Cube4`) "Socket" "SnapToTarget" "SnapToTarget" "SnapToTarget" true)
                (set `self.Is Holding` true)
                (`/Game/Menus_And_Widgets/W_Inventory.AddItem` (`self.Inventory`) (castclass `/Game/Blueprints/Items/BP_ItemTest_P` (`GameplayStatics.GetObjectClass` _array_element) :!pure true))
                (`KismetSystemLibrary.PrintString` "Held")
                (break)))))))))

(event `KeyPickUpItemFunction`
  ;[1 1 1] Pick Up Item
  (goto _label))

(event `KeyDropItemFuntion`
  ;[1 1 1] DropItem (Key Version)
  (goto _label_3))

(event `Pick Up Weeds`
  ;[1 1 1] Pick Up Weeds
  (set `self.HoldingWeed` true)
  (for _array_element (`self.GetOverlappingActors` "/Game/Blueprints/Items/Weeds/BP_Item_Weeds_P.BP_Item_Weeds_P_C")
    ;;[1 1 1] Max Amoutn Weeds that can be Carried
    (if (== (`KismetArrayLibrary.Array_Length` (`self.WeedsHeld`)) 3)
      _
      (elif (`self.ActorHasTag` _array_element "Weed")
        ;;[1 1 1] Adds Weed to Array when Picked Up
        (`KismetArrayLibrary.Array_Add` (`self.WeedsHeld`) _array_element)
        (`KismetSystemLibrary.PrintString` "Weed in bag")
        (`self.K2_DestroyActor` (`self.GetOverlappingActors` "/Game/Blueprints/Items/Weeds/BP_Item_Weeds_P.BP_Item_Weeds_P_C"))
        (break)))))

(event `InputAction|Pick Up (E)`
  (params (Key :type "Key Structure"))
  ;[1 1 1] Basic Garbage Bin Function (Clears Weeds in Garbage Bag)
  (:`Pressed`
    (if (`self.HoldingWeed`)
      (for _ (`self.GetOverlappingActors` "/Game/Blueprints/Items/Weeds/BP_GarbageBin.BP_GarbageBin_C")
        (`KismetArrayLibrary.Array_Clear` (`self.WeedsHeld`))
        ;;[1 1 1] Ensures it Activates Second and clears the weeds from the bag
        (`KismetSystemLibrary.Delay` 0.5)
        (set `self.HoldingWeed` false)
        (break)))))

(event `Create Garbage Bag Array`
  ;[1 1 1] Amount Garbage Bag Can Store
  (if (`self.Is Holding Garbage`)
    (bind _output_get (set `self.WeedsHeld` (`self.WeedsHeld`)))
    (`KismetArrayLibrary.Array_Set` _output_get 3)
    (if (`self.InventoryActive`)
      (`/Game/Menus_And_Widgets/W_Inventory.CreateWeedWidget` (`self.Inventory`)))))

(event `InputAction|ToggleInventory (I)`
  (params (Key :type "Key Structure"))
  (bind _inventory (`self.Inventory`))
  ;[1 1 1] Inventory Toggle
  ;;[1 1 1] Input Action Cant be Called like other events
  (:`Pressed`
    ;;[1 1 1] No Clue Why this is need for the inventory to Operate. But it is needed
    (if (not (`self.InGameMenuActive`))
      (if (not (`Widget.IsInViewport` (`self.Inventory`))) :!label _label_5
        (`/Game/Menus_And_Widgets/W_Inventory.SetupInvetory` _inventory "I")
        (`/Game/Menus_And_Widgets/W_Inventory.Show` _inventory)
        (set `self.InventoryActive` true)))))

(event `self.ReceiveBeginPlay`
  ;[1 1 1] Ensures Inventory Widget is waiting to be added to ViewPort
  (bind _returnvalue (`|CreateWidget` "/Game/Menus_And_Widgets/W_InGameMenu.W_InGameMenu_C" (`GameplayStatics.GetPlayerController` 0)))
  (set `self.InGameMenu` _returnvalue)
  (bind _returnvalue_2 (`|CreateWidget` "/Game/Menus_And_Widgets/W_Inventory.W_Inventory_C" (`GameplayStatics.GetPlayerController` 0)))
  (set `self.Inventory` _returnvalue_2)
  (`|ExecutionSequence`
    (:`then_0`
      (`/Engine/EditorBlueprintResources/StandardMacros.DoOnce` false
        (:`Completed`
          (`KismetSystemLibrary.Delay` 1.0)
          (goto _label_5))))
    (:`then_1`
      (bind _returnvalue_3 (`|CreateWidget` "/Game/Menus_And_Widgets/W_MemorialInterface.W_MemorialInterface_C" (`GameplayStatics.GetPlayerController` 0) null))
      (set `self.MemorialInterface` _returnvalue_3))))

(event `self.ReceiveTick`
  (params (DeltaSeconds :type "Float (single-precision)"))
  ;[1 1 1] Activate Cycle (BED)
  (bind _returnvalue (`GameplayStatics.GetActorOfClass` "/Game/Blueprints/DayNightCycle/NOTINUSE_BP_TempBedActor.NOTINUSE_BP_TempBedActor_C")))

(event `InputAction|Pause Game (Q)`
  (params (Key :type "Key Structure"))
  ;[1 1 1] Pause Game
  (:`Pressed`
    (if (`self.IsOverlappingActor` self (stale `self.ReceiveTick` _returnvalue))
      ;[1 1 1] True Activates after First Cycle
      (if (`self.SpawnedFirstMemoryBox`)
        (set `self.SetDay2` true)
        (`KismetSystemLibrary.PrintString` "SetSpawned2Bool")
        ;[1 1 1] Need to cast for 2nd save to Work
        (bind _asgame_mode_load_save_1 (cast `/Game/Blueprints/SaveBluePrints/GameModeLoad_Save_1` (`GameplayStatics.GetGameMode`))
          (:`then`
            (`/Game/Blueprints/SaveBluePrints/GameModeLoad_Save_1.SetDay2` _asgame_mode_load_save_1)
            ;[1 1 1] Activate Cycle (BED)
            (bind _returnvalue (`GameplayStatics.GetCurrentLevelName` true :!label _label_6))
            (`GameplayStatics.OpenLevel` (`KismetStringLibrary.Conv_StringToName` _returnvalue)))
          (:`CastFailed`
            (`KismetSystemLibrary.PrintString` "fail 2")))
        (else
          (set `self.SpawnedFirstMemoryBox` true)
          (`KismetSystemLibrary.PrintString` "SetSpawned1Bool")
          (bind _asgame_mode_load_save_1_2 (cast `/Game/Blueprints/SaveBluePrints/GameModeLoad_Save_1` (`GameplayStatics.GetGameMode`))
            (:`then`
              (`/Game/Blueprints/SaveBluePrints/GameModeLoad_Save_1.SaveBoxSet1` _asgame_mode_load_save_1_2)
              (goto _label_6))
            (:`CastFailed`
              (`KismetSystemLibrary.PrintString` "FAIL 1")))))
      (else
        (`KismetSystemLibrary.PrintString` "ActionButtonq")
        (if (not (`Widget.IsInViewport` (`self.InGameMenu`)))
          (`/Game/Menus_And_Widgets/W_InGameMenu.ShowMenu` (`self.InGameMenu`))
          (set `self.InGameMenuActive` true)
          (`Widget.RemoveFromParent` (`self.Inventory`))
          (set `self.InventoryActive` false))))))

(event `Create Memorial Items Set 1`
  ;[1 1 1] Adds items to Memorial Inventory when level start. V1
  (if (`self.SpawnedFirstMemoryBox`)
    (`KismetSystemLibrary.PrintString` "BOX 1 NO SPAWN")
    (if (`self.SetDay2`)
      (`KismetSystemLibrary.PrintString` "DAY 2")
      ;[1 1 1] Adds items to Memorial Inventory when level start. V2
      (if (`self.SpawnedSecondMemoryBox`) :!label _label_7
        (`KismetSystemLibrary.PrintString` "No BOX 2")
        (else
          (`/Engine/EditorBlueprintResources/StandardMacros.DoOnce` false
            (:`Completed`
              (`|ExecutionSequence`
                (:`then_0`
                  (for _array_element (`self.Memorial Items Set 2`)
                    (`/Game/Menus_And_Widgets/W_MemorialInterface.AddMemorialItem` (`self.MemorialInterface`) _array_element)
                    (set `self.SpawnedSecondMemoryBox` true)))
                (:`then_1`
                  ;[1 1 1] Adds items to Memorial Inventory when Level Start. V2
                  (`KismetSystemLibrary.PrintString` "BOX 2 sET")
                  (set `self.SpawnedSecondMemoryBox` true)
                  (bind _asgame_mode_load_save_1 (cast `/Game/Blueprints/SaveBluePrints/GameModeLoad_Save_1` (`GameplayStatics.GetGameMode`)))
                  (`/Game/Blueprints/SaveBluePrints/GameModeLoad_Save_1.SaveBoxSet2` _asgame_mode_load_save_1))))))))
    (else
      (`KismetSystemLibrary.PrintString` "BOX 1 SPAWN")
      (`/Engine/EditorBlueprintResources/StandardMacros.DoOnce` false
        (:`Completed`
          (`|ExecutionSequence`
            (:`then_0`
              (for _array_element_2 (`self.Memorial Items Set 1`)
                (if true
                  (`/Game/Menus_And_Widgets/W_MemorialInterface.AddMemorialItem` (`self.MemorialInterface`) _array_element_2)
                  (`KismetSystemLibrary.PrintString` "Hello1"))))
            (:`then_1`
              ;[1 1 1] Adds items to Memorial Inventory when Level Start. V1
              (`KismetSystemLibrary.PrintString` "BOX sET")
              (set `self.SpawnedFirstMemoryBox` true)
              (bind _asgame_mode_load_save_1_2 (cast `/Game/Blueprints/SaveBluePrints/GameModeLoad_Save_1` (`GameplayStatics.GetGameMode`)))
              (`/Game/Blueprints/SaveBluePrints/GameModeLoad_Save_1.SaveBoxSet1` _asgame_mode_load_save_1_2)
              (`KismetSystemLibrary.PrintString` "Hello2"))))))))

(event `Create Memorial Items Set 2`
  ;[1 1 1] Not in use Kept just incase
  (goto _label_7))

(event `Reposition Memorial Item Pick Up`
  (bind (_worldlocation _worlddirection) (`PlayerController.DeprojectMousePositionToWorld` (`GameplayStatics.GetPlayerController` 0)))
  ;[1 1 1] Allows Memorial Items to be pickd up by Click
  ;;[1 1 1] Gets the in world Mouse Poistion
  (bind _outhit (`KismetSystemLibrary.LineTraceSingle` _worldlocation (+ _worldlocation (* _worlddirection 10000.0)) "TraceTypeQuery1"))
  (bind (_bblockinghit _binitialoverlap _time _distance _location _impactpoint _normal _impactnormal _physmat _hitactor) (`GameplayStatics.BreakHitResult` _outhit))
  (if (`self.ActorHasTag` _hitactor "PickUpAble")
    (if (`self.ActorHasTag` _hitactor "MemoryItem")
      (`/Game/Menus_And_Widgets/W_MemorialInterface.AddMemorialItem` (`self.MemorialInterface`) (castclass `/Game/Blueprints/Items/BP_ItemTest_P` (`GameplayStatics.GetObjectClass` _hitactor) :!pure true))
      (`self.K2_DestroyActor` _hitactor))))

(event `InputAction|ActivateGraveCamera (F)`
  (params (Key :type "Key Structure"))
  (bind _returnvalue (`GameplayStatics.GetPlayerController` 0))
  ;[1 1 1] Activate Grave Camera and Setup
  (:`Pressed`
    (if (not (`Widget.IsInViewport` (`self.GraveCameraInterfaceLeave`)))
      (if (`self.IsHoldingMemoryBox`)
        (if (`self.Is OverlapingWithGraveActivation`)
          ;;[1 1 1] Redundant
          (`MovementComponent.StopMovementImmediately` (`self.CharacterMovement`))
          (`Controller.StopMovement` _returnvalue)
          ;;[1 1 1] Will definitly stop player
          (`Controller.SetIgnoreMoveInput` _returnvalue true))))))

(event `self.ReceiveActorBeginOverlap`
  (params (OtherActor :type "Actor Object Reference"))
  (cast `/Game/Blueprints/Graves_MemorialGrid/BP_Camera_Activation_Braum` OtherActor)
  (set `self.Is OverlapingWithGraveActivation` true))

(event `self.ReceiveActorEndOverlap`
  (params (OtherActor :type "Actor Object Reference"))
  (cast `/Game/Blueprints/Graves_MemorialGrid/BP_Camera_Activation_Braum` OtherActor)
  (set `self.Is OverlapingWithGraveActivation` false))

(event `InputAction|TempTestKey (G)`
  (params (Key :type "Key Structure"))
  ;[1 1 1] Under Construction
)

(fn `UserConstructionScript`)