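; Watering can hold-item Blueprint, a child item that can show and hide an on-screen info widget.
; ShowWidgetCAN creates a W_InforWidget_GarbageBin, the garbage bin's info widget class, and adds it to the viewport.
; RemoveWIDGETCAN removes that created widget from its parent.
; BeginPlay, overlap and Tick are disabled stubs, and the construction script only calls the parent.
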(event `Show WidgetCAN`
  (bind _returnvalue (`|CreateWidget` "/Game/Menus_And_Widgets/W_InforWidget_GarbageBin.W_InforWidget_GarbageBin_C"))
  (`UserWidget.AddToViewport` _returnvalue 0))

(event `RemoveWIDGETCAN`
  (`Widget.RemoveFromParent` (stale `Show WidgetCAN` _returnvalue)))

(fn `UserConstructionScript`
  (`parent.UserConstructionScript`))