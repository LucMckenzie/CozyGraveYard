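; BP_WEED_SPAWNManager is a manager that scatters instances of a configurable actor class, presumably weeds, across the level's Target Points when play begins.
; It gathers every TargetPoint in the level, then spawns ActorCount actors at randomly picked points, removing each used point so picks do not repeat.
; Spawning ignores collision, and a debug message prints if no Target Points exist.
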(event `self.ReceiveBeginPlay`
  (bind _actorcount (`self.actorCount`))
  (bind _outactors (`GameplayStatics.GetAllActorsOfClass` "/Script/Engine.TargetPoint"))
  (set `self.placesToSpawn` _outactors)
  (if (> (`KismetArrayLibrary.Array_Length` (`self.placesToSpawn`)) 0)
    (`/Engine/EditorBlueprintResources/StandardMacros.DecrementInt` _actorcount
      (:`  `
        (for _ (range (+ _actorcount 1))
          (bind _output_get (set `self.currentSpawnPoint` (`KismetArrayLibrary.Array_Random` (`self.placesToSpawn`))))
          (`|SpawnActorFromClass` (`self.actorToSpawn`) (`self.GetTransform` _output_get) "AlwaysSpawn" "OverrideRootScale" null null)
          (`KismetArrayLibrary.Array_RemoveItem` (`self.placesToSpawn`) (`self.currentSpawnPoint`)))))
    (else
      (`KismetSystemLibrary.PrintString` "Forgot to set places to Spawn, lenght is 0"))))

(fn `UserConstructionScript`)