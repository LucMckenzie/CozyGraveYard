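; BP_ItemTest_Child_MemoryItem_P is a child item Blueprint for a clickable memorial item pickup.
; Clicking its StaticMechComp casts the player character to BP_TestPlayerCharacter2 and, if MemorialCameraActive is set, calls RepositionMemorialItemPickUp and destroys the item.
; Disconnected, under-construction nodes sketch saving the item and its transform through GameModeLoadSave1, but never run.
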(event `self.StaticMechComp.OnClicked`
  (params (TouchedComponent :type "PrimitiveComponent Object Reference") (ButtonPressed :type "Key Structure"))
  (bind _asbp_test_player_character_2 (cast `/Game/Blueprints/Character/BP_TestPlayerCharacter2` (`GameplayStatics.GetPlayerCharacter` 0)))
  (if (`/Game/Blueprints/Character/BP_TestPlayerCharacter2.MemorialCameraActive` _asbp_test_player_character_2)
    (`/Game/Blueprints/Character/BP_TestPlayerCharacter2.Reposition Memorial Item Pick Up` _asbp_test_player_character_2)
    (`self.K2_DestroyActor`)))

(fn `UserConstructionScript`
  (`parent.UserConstructionScript`))