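; BP_SingleActor_SpawnManager is a spawn manager that places ActorCount copies of a single ActorToSpawn class in the level on BeginPlay.
; Each loop pass spawns at the first PlacesToSpawn entry's transform, then removes CurrentSpawnPoint, a variable never assigned in these graphs, from the list.
; An empty list prints a warning instead.
; Unconnected leftover nodes would gather TargetPoints automatically and check the actor count.
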(event `self.ReceiveBeginPlay`
  (if (> (`KismetArrayLibrary.Array_Length` (`self.placesToSpawn`)) 0)
    (for _ (range 1 (+ (`self.actorCount`) 1))
      (`|SpawnActorFromClass` (`self.actorToSpawn`) (`self.GetTransform` (`|GetArrayItem` (`self.placesToSpawn`))) "Undefined" "OverrideRootScale" null null)
      (`KismetArrayLibrary.Array_RemoveItem` (`self.placesToSpawn`) (`self.currentSpawnPoint`)))
    (else
      (`KismetSystemLibrary.PrintString` "Forgot to set places to Spawn, lenght is 0"))))

(fn `UserConstructionScript`)