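; Work-in-progress game instance that resets saved progress when a new game starts.
; StartNewGameMode loads the Game1SaveVariables save from a slot named after the main menu widget's OpenLevel class default.
; It clears the JaneDoe and BramBox spawn flags, the day 2 and 3 flags, and the memorial item location and object collections, then saves to the same slot.
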(event `StartNewGameMode`
  (bind _returnvalue (`GameplayStatics.LoadGameFromSlot` (`KismetStringLibrary.Conv_NameToString` (defaults `Object` (castclass `/Game/Menus_And_Widgets/W_MainMenu` "/Game/Menus_And_Widgets/W_MainMenu.W_MainMenu_C" :!pure true)))))
  (bind _asgame_1save_variables (cast `/Game/Blueprints/SaveBluePrints/Game1SaveVariables` _returnvalue :!pure true))
  (set `/Game/Blueprints/SaveBluePrints/Game1SaveVariables.JaneDoeSpawned` false _asgame_1save_variables)
  (set `/Game/Blueprints/SaveBluePrints/Game1SaveVariables.BramBoxSpawned` false _asgame_1save_variables)
  (set `/Game/Blueprints/SaveBluePrints/Game1SaveVariables.Set Day 2` false _asgame_1save_variables)
  (set `/Game/Blueprints/SaveBluePrints/Game1SaveVariables.Set Day 3` false _asgame_1save_variables)
  (`BlueprintMapLibrary.Map_Clear` (`/Game/Blueprints/SaveBluePrints/Game1SaveVariables.MemorialItemLocation` _asgame_1save_variables))
  (`KismetArrayLibrary.Array_Clear` (`/Game/Blueprints/SaveBluePrints/Game1SaveVariables.ObjectList` _asgame_1save_variables))
  (`GameplayStatics.GetCurrentLevelName` true)
  (`GameplayStatics.SaveGameToSlot` _asgame_1save_variables (`KismetStringLibrary.Conv_NameToString` (defaults `Object` (castclass `/Game/Menus_And_Widgets/W_MainMenu` "/Game/Menus_And_Widgets/W_MainMenu.W_MainMenu_C" :!pure true)))))