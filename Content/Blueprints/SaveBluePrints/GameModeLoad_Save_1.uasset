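; Game mode Blueprint that manages per-level save data for memory item actors, using the current level name as the slot name.
; On BeginPlay it loads or creates a Game1SaveVariables object.
; SaveLevelData refills FailedAttempt1 with every BP_ItemTest_Child_MemoryItem_P transform, writing to disk inside the loop, so nothing is written when none exist.
; Saved items are never respawned; the spawn and MemorialItemLocation map logic is disconnected.
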(event `self.ReceiveBeginPlay`
  (`self.InitLevelSaveData`))

(fn `InitLevelSaveData`
  (bind _returnvalue (`GameplayStatics.GetCurrentLevelName` true))
  (bind _returnvalue_2 (`GameplayStatics.DoesSaveGameExist` _returnvalue))
  (if _returnvalue_2
    (bind _returnvalue_3 (`GameplayStatics.GetCurrentLevelName` true))
    (bind _returnvalue_4 (`GameplayStatics.LoadGameFromSlot` _returnvalue_3))
    (bind _asgame_1save_variables (cast `/Game/Blueprints/SaveBluePrints/Game1SaveVariables` _returnvalue_4))
    (set `self.Game1_SaveVariables` _asgame_1save_variables)
    (else
      (bind _returnvalue_5 (`GameplayStatics.CreateSaveGameObject` "/Game/Blueprints/SaveBluePrints/Game1SaveVariables.Game1SaveVariables_C"))
      (set `self.Game1_SaveVariables` _returnvalue_5))))

(fn `SaveLevelData`
  (bind _failedattempt1 (`/Game/Blueprints/SaveBluePrints/Game1SaveVariables.FailedAttempt1` (`self.Game1_SaveVariables`)))
  (`KismetArrayLibrary.Array_Clear` _failedattempt1)
  (bind _outactors (`GameplayStatics.GetAllActorsOfClass` "/Game/Blueprints/Items/BP_ItemTest_Child_MemoryItem_P.BP_ItemTest_Child_MemoryItem_P_C"))
  (for _array_element _outactors
    (`KismetArrayLibrary.Array_Add` _failedattempt1 (`self.GetTransform` _array_element))
    (bind _returnvalue (`GameplayStatics.GetCurrentLevelName` true))
    (`GameplayStatics.SaveGameToSlot` (`self.Game1_SaveVariables`) _returnvalue)))

(fn `UserConstructionScript`)