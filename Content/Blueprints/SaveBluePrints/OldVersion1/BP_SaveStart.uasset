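; BP_SaveStart is a level-transition trigger that records its use in the save data and removes a portal on later loads.
; On overlap it sets its indexed flag in BP_SaveVariables' bool array, saves through BP_GameInstance and opens the named level.
; On BeginPlay it destroys the referenced target actor if that flag is set, so only that specific portal disappears.
; Debug prints trace both paths.
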(event `self.ReceiveBeginPlay`
  ;[1 1 1] Destory Portal if Variable Set
  (bind _asbp_game_instance (cast `/Game/Blueprints/SaveBluePrints/OldVersion1/BP_GameInstance` (`GameplayStatics.GetGameInstance`)))
  (bind _asbp_save_variables (cast `/Game/Blueprints/SaveBluePrints/OldVersion1/BP_SaveVariables` (`/Game/Blueprints/SaveBluePrints/OldVersion1/BP_GameInstance.SaveGameData` _asbp_game_instance)))
  (if (`|GetArrayItem` (`/Game/Blueprints/SaveBluePrints/OldVersion1/BP_SaveVariables.SaveInfoBool` _asbp_save_variables) (`self.Index`))
    (`KismetSystemLibrary.PrintString` "Destroy")
    ;;[1 1 1] Target needed to ensure only one Specific portal is Destoryed. Otherwise all are Destroyed
    (`self.K2_DestroyActor` (`self.TestDestroyObject`))
    (`KismetSystemLibrary.PrintString` "DestroyWorked")))

(event `self.ReceiveActorBeginOverlap`
  (params (OtherActor :type "Actor Object Reference"))
  (bind _asbp_game_instance (cast `/Game/Blueprints/SaveBluePrints/OldVersion1/BP_GameInstance` (`GameplayStatics.GetGameInstance`))
    (:`then`
      (`KismetSystemLibrary.PrintString` "Hello")
      (bind _asbp_save_variables (cast `/Game/Blueprints/SaveBluePrints/OldVersion1/BP_SaveVariables` (`/Game/Blueprints/SaveBluePrints/OldVersion1/BP_GameInstance.SaveGameData` _asbp_game_instance))
        (:`then`
          (`KismetSystemLibrary.PrintString` "Hello2 ")
          (`KismetArrayLibrary.Array_Set` (`/Game/Blueprints/SaveBluePrints/OldVersion1/BP_SaveVariables.SaveInfoBool` _asbp_save_variables) (`self.Index`) true)
          (`/Game/Blueprints/SaveBluePrints/OldVersion1/BP_GameInstance.Save` _asbp_game_instance)
          (`GameplayStatics.OpenLevel` (`self.Level Name`)))
        (:`CastFailed`
          (`KismetSystemLibrary.PrintString` "Hello 1"))))
    (:`CastFailed`
      (`KismetSystemLibrary.PrintString` "Hello"))))

(fn `UserConstructionScript`)