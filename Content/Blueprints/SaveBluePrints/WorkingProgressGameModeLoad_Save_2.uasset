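; Game mode that saves and loads per-level progress in a save game slot named after the current level.
; BeginPlay loads or creates the save object, then a sequence restores player memory-box and day flags, respawns memorial items, and refills the memorial inventory after a short delay.
; Separate functions write each flag, item transforms and inventory classes, or reset everything.
; Transforms are keyed by class, so only one per item class persists.
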(event `self.ReceiveBeginPlay`
  (`self.InitLevelSaveData`)
  (`self.Load`))

(event `Load`
  (bind _memorialitemlocation (`/Game/Blueprints/SaveBluePrints/Game1SaveVariables.MemorialItemLocation` (`.Game2_SaveVariables` (`self.Game2_SaveVariables`))))
  ;[1 1 1] Sequenced so I know when what loads when and so there is no bottle neck
  (`|ExecutionSequence`
    (:`then_0`
      (bind _asbp_test_player_character_2 (cast `/Game/Blueprints/Character/BP_TestPlayerCharacter2` (`GameplayStatics.GetPlayerCharacter` 0)))
      (set `/Game/Blueprints/Character/BP_TestPlayerCharacter2.SpawnedMemoryBoxBraum` (`/Game/Blueprints/SaveBluePrints/Game1SaveVariables.BramBoxSpawned` (`.Game2_SaveVariables` (`self.Game2_SaveVariables`))) _asbp_test_player_character_2))
    (:`then_1`
      (bind _asbp_test_player_character_2_2 (cast `/Game/Blueprints/Character/BP_TestPlayerCharacter2` (`GameplayStatics.GetPlayerCharacter` 0)))
      (set `/Game/Blueprints/Character/BP_TestPlayerCharacter2.SetDay3` (`/Game/Blueprints/SaveBluePrints/Game1SaveVariables.Set Day 3` (`.Game2_SaveVariables` (`self.Game2_SaveVariables`))) _asbp_test_player_character_2_2))
    (:`then_2`
      (bind _asbp_test_player_character_2_3 (cast `/Game/Blueprints/Character/BP_TestPlayerCharacter2` (`GameplayStatics.GetPlayerCharacter` 0)))
      (set `/Game/Blueprints/Character/BP_TestPlayerCharacter2.SetDay2` (`/Game/Blueprints/SaveBluePrints/Game1SaveVariables.Set Day 2` (`.Game2_SaveVariables` (`self.Game2_SaveVariables`))) _asbp_test_player_character_2_3))
    (:`then_3`
      (bind _asbp_test_player_character_2_4 (cast `/Game/Blueprints/Character/BP_TestPlayerCharacter2` (`GameplayStatics.GetPlayerCharacter` 0)))
      (set `/Game/Blueprints/Character/BP_TestPlayerCharacter2.SpawnedMemoryBoxJaneDoe` (`/Game/Blueprints/SaveBluePrints/Game1SaveVariables.JaneDoeSpawned` (`.Game2_SaveVariables` (`self.Game2_SaveVariables`))) _asbp_test_player_character_2_4))
    (:`then_4`
      (bind _keys (`BlueprintMapLibrary.Map_Keys` _memorialitemlocation))
      (for _array_element _keys
        (`|SpawnActorFromClass` _array_element (`BlueprintMapLibrary.Map_Find` _memorialitemlocation _array_element) "Undefined" "OverrideRootScale" null null)))
    (:`then_5`
      (`KismetSystemLibrary.Delay` 0.2)
      (bind _asbp_test_player_character_2_5 (cast `/Game/Blueprints/Character/BP_TestPlayerCharacter2` (`GameplayStatics.GetPlayerCharacter` 0))
        (:`then`
          ;[1 1 1] Takes saved variables (Class)Item_Test_P (Will add wrong amount of Objects and the dont contain the correct data)
          (for _array_element_2 (`/Game/Blueprints/SaveBluePrints/Game1SaveVariables.ObjectList` (`.Game2_SaveVariables` (`self.Game2_SaveVariables`)))
            (`/Game/Menus_And_Widgets/W_MemorialInterface.LoadAddMemorialItem` (`/Game/Blueprints/Character/BP_TestPlayerCharacter2.MemorialInterface` _asbp_test_player_character_2_5) _array_element_2)))
        (:`CastFailed`
          (`KismetSystemLibrary.PrintString` "Failed Load Objects"))))))

(fn `InitLevelSaveData`
  (bind _returnvalue (`GameplayStatics.GetCurrentLevelName` true))
  (bind _returnvalue_2 (`GameplayStatics.DoesSaveGameExist` _returnvalue))
  (if _returnvalue_2
    (bind _returnvalue_3 (`GameplayStatics.GetCurrentLevelName` true))
    (bind _returnvalue_4 (`GameplayStatics.LoadGameFromSlot` _returnvalue_3))
    (bind _asgame_2save_variables (cast `/Game/Blueprints/SaveBluePrints/WorkingProgressGame2SaveVariables` _returnvalue_4))
    (set `self.Game2_SaveVariables` _asgame_2save_variables)
    (else
      (bind _returnvalue_5 (`GameplayStatics.CreateSaveGameObject` "/Game/Blueprints/SaveBluePrints/WorkingProgressGame2SaveVariables.WorkingProgressGame2SaveVariables_C"))
      (set `self.Game2_SaveVariables` _returnvalue_5))))

(fn `Reset`
  (bind (_game1_savevariables _game2_savevariables) (`self.Game2_SaveVariables`))
  (bind _returnvalue (`GameplayStatics.GetCurrentLevelName` true))
  (`GameplayStatics.LoadGameFromSlot` _returnvalue)
  (set `/Game/Blueprints/SaveBluePrints/Game1SaveVariables.JaneDoeSpawned` false _game2_savevariables)
  (set `/Game/Blueprints/SaveBluePrints/Game1SaveVariables.BramBoxSpawned` false _game2_savevariables)
  (set `/Game/Blueprints/SaveBluePrints/Game1SaveVariables.Set Day 2` false _game2_savevariables)
  (set `/Game/Blueprints/SaveBluePrints/Game1SaveVariables.Set Day 3` false _game2_savevariables)
  (`BlueprintMapLibrary.Map_Clear` (`/Game/Blueprints/SaveBluePrints/Game1SaveVariables.MemorialItemLocation` _game2_savevariables))
  (`KismetArrayLibrary.Array_Clear` (`/Game/Blueprints/SaveBluePrints/Game1SaveVariables.ObjectList` _game2_savevariables))
  (bind _returnvalue_2 (`GameplayStatics.GetCurrentLevelName` true))
  (`GameplayStatics.SaveGameToSlot` _game2_savevariables _returnvalue_2))

(fn `SaveBoxSet1`
  (bind (_game1_savevariables _game2_savevariables) (`self.Game2_SaveVariables`))
  (bind _asbp_test_player_character_2 (cast `/Game/Blueprints/Character/BP_TestPlayerCharacter2` (`GameplayStatics.GetPlayerCharacter` 0)))
  (set `/Game/Blueprints/SaveBluePrints/Game1SaveVariables.BramBoxSpawned` (`/Game/Blueprints/Character/BP_TestPlayerCharacter2.SpawnedMemoryBoxBraum` _asbp_test_player_character_2) _game2_savevariables)
  (bind _returnvalue (`GameplayStatics.GetCurrentLevelName` true))
  (`GameplayStatics.SaveGameToSlot` _game2_savevariables _returnvalue)
  (`KismetSystemLibrary.PrintString` "Box 1 Data Saved"))

(fn `SaveBoxSet2`
  (bind (_game1_savevariables _game2_savevariables) (`self.Game2_SaveVariables`))
  (bind _asbp_test_player_character_2 (cast `/Game/Blueprints/Character/BP_TestPlayerCharacter2` (`GameplayStatics.GetPlayerCharacter` 0)))
  (set `/Game/Blueprints/SaveBluePrints/Game1SaveVariables.JaneDoeSpawned` (`/Game/Blueprints/Character/BP_TestPlayerCharacter2.SpawnedMemoryBoxJaneDoe` _asbp_test_player_character_2) _game2_savevariables)
  (bind _returnvalue (`GameplayStatics.GetCurrentLevelName` true))
  (`GameplayStatics.SaveGameToSlot` _game2_savevariables _returnvalue)
  (`KismetSystemLibrary.PrintString` "Box 2 Data Saved "))

(fn `SaveLevelData`
  (bind _memorialitemlocation (`/Game/Blueprints/SaveBluePrints/Game1SaveVariables.MemorialItemLocation` (`.Game2_SaveVariables` (`self.Game2_SaveVariables`))))
  (`BlueprintMapLibrary.Map_Clear` _memorialitemlocation)
  (bind _outactors (`GameplayStatics.GetAllActorsOfClass` "/Game/Blueprints/Items/BP_ItemTest_Child_MemoryItem_P.BP_ItemTest_Child_MemoryItem_P_C"))
  (for _array_element _outactors
    (`BlueprintMapLibrary.Map_Add` _memorialitemlocation (`GameplayStatics.GetObjectClass` _array_element) (`self.GetTransform` _array_element))
    (bind _returnvalue (`GameplayStatics.GetCurrentLevelName` true))
    (`GameplayStatics.SaveGameToSlot` (`self.Game2_SaveVariables`) _returnvalue)
    (`KismetSystemLibrary.PrintString` "Location Data Save")))

(fn `SaveMemorialInventory`
  ;[1 1 1] Gets items from Memorial Interface
  (bind _asbp_test_player_character_2 (cast `/Game/Blueprints/Character/BP_TestPlayerCharacter2` (`GameplayStatics.GetPlayerCharacter` 0)))
  (`KismetArrayLibrary.Array_Clear` (`/Game/Blueprints/SaveBluePrints/Game1SaveVariables.ObjectList` (`.Game2_SaveVariables` (`self.Game2_SaveVariables`))))
  (for _array_element (`ListView.GetListItems` (`/Game/Menus_And_Widgets/W_MemorialInterface.TileView_170` (`/Game/Blueprints/Character/BP_TestPlayerCharacter2.MemorialInterface` _asbp_test_player_character_2)))
    (bind _asbp_item_object_p (cast `/Game/Blueprints/Items/BP_ItemObject_P` _array_element))
    (`KismetArrayLibrary.Array_AddUnique` (`/Game/Blueprints/SaveBluePrints/Game1SaveVariables.ObjectList` (`.Game2_SaveVariables` (`self.Game2_SaveVariables`))) (`/Game/Blueprints/Items/BP_ItemObject_P.ItemClass` _asbp_item_object_p)))
  ;[1 1 1] Saves them as ItemTest_P (Converts?)
  (bind _returnvalue (`GameplayStatics.GetCurrentLevelName` true))
  (`GameplayStatics.SaveGameToSlot` (`.Game2_SaveVariables` (`self.Game2_SaveVariables`)) _returnvalue)
  (`KismetSystemLibrary.PrintString` "SaveInventory"))

(fn `SetDay2`
  (bind (_game1_savevariables _game2_savevariables) (`self.Game2_SaveVariables`))
  (bind _asbp_test_player_character_2 (cast `/Game/Blueprints/Character/BP_TestPlayerCharacter2` (`GameplayStatics.GetPlayerCharacter` 0)))
  (set `/Game/Blueprints/SaveBluePrints/Game1SaveVariables.Set Day 2` (`/Game/Blueprints/Character/BP_TestPlayerCharacter2.SetDay2` _asbp_test_player_character_2) _game2_savevariables)
  (bind _returnvalue (`GameplayStatics.GetCurrentLevelName` true))
  (`GameplayStatics.SaveGameToSlot` _game2_savevariables _returnvalue)
  (`KismetSystemLibrary.PrintString` "DAY 2 Data Saved "))

(fn `SetDay3`
  (bind (_game1_savevariables _game2_savevariables) (`self.Game2_SaveVariables`))
  (bind _asbp_test_player_character_2 (cast `/Game/Blueprints/Character/BP_TestPlayerCharacter2` (`GameplayStatics.GetPlayerCharacter` 0)))
  (set `/Game/Blueprints/SaveBluePrints/Game1SaveVariables.Set Day 3` (`/Game/Blueprints/Character/BP_TestPlayerCharacter2.SetDay3` _asbp_test_player_character_2) _game2_savevariables)
  (bind _returnvalue (`GameplayStatics.GetCurrentLevelName` true))
  (`GameplayStatics.SaveGameToSlot` _game2_savevariables _returnvalue)
  (`KismetSystemLibrary.PrintString` "DAY 3  Data Saved "))

(fn `UserConstructionScript`)