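; Grid manager actor, named as reference-only, that spawns ForReferenceOnly_GridCell actors at BeginPlay and offers a position-snap function.
; PopulateGrid stores cells in GridArray, spaced by WorldGridSize with a world-origin centring offset, but its Y loop covers only the last row.
; GridSnap is structured as a nearest-cell search, but compares cells against the current closest position instead of Input, so it returns the first cell's location.
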(event `self.ReceiveBeginPlay`
  (`self.PopulateGrid`))

(fn `GridSnap`
  (params (Input :type "Vector Structure"))
  (returns (Output :type "Vector Structure"))
  (locals (`Closest Position ` :type "Vector Structure") (`Closest Distance` :type "Float (double-precision)"))
  (bind _returnvalue (`self.K2_GetActorLocation` (`|GetArrayItem` (`self.GridArray`))))
  (bind _output_get (set `local.Closest Position ` _returnvalue))
  (set `local.Closest Distance` (`KismetMathLibrary.Vector_Distance` Input _returnvalue))
  (for _array_element (`self.GridArray`)
    (bind _returnvalue_2 (`self.K2_GetActorLocation` _array_element))
    (bind _returnvalue_3 (`KismetMathLibrary.Vector_Distance` _returnvalue_2 _output_get))
    (if (< _returnvalue_3 (`local.Closest Distance`))
      (set `local.Closest Position ` _returnvalue_2)
      (set `local.Closest Distance` _returnvalue_3)))
  (return (`local.Closest Position `)))

(fn `PopulateGrid`
  (locals (WorldOffSet :type "Float (double-precision)"))
  (bind _worldgridsize (`self.WorldGridSize`))
  (bind _worldgridsize_2 (`self.WorldGridSize`))
  (bind _worldoffset (`local.WorldOffSet`))
  (bind _returnvalue (- (`self.GridSize`) 1))
  (`KismetArrayLibrary.Array_Clear` (`self.GridArray`))
  (set `local.WorldOffSet` (- (* (* (`self.GridSize`) _worldgridsize) 0.5) (* _worldgridsize 0.5)))
  ;[1 1 1] Y Loop
  (for _index (range _returnvalue (+ _returnvalue 1))
    ;[1 1 1] X Loop
    (for _index_2 (range (`self.GridSize`))
      (bind _returnvalue_2 (`|SpawnActorFromClass` "/Game/Blueprints/MemorialGrid/ForReferenceOnly_GridCell.ForReferenceOnly_GridCell_C" (`KismetMathLibrary.MakeTransform` (`KismetMathLibrary.MakeVector` (`KismetMathLibrary.Conv_IntToDouble` (- (* _index_2 _worldgridsize_2) (`KismetMathLibrary.FTrunc` _worldoffset))) (`KismetMathLibrary.Conv_IntToDouble` (- (* _worldgridsize_2 _index) (`KismetMathLibrary.FTrunc` _worldoffset))))) "Undefined" "OverrideRootScale" null null))
      (`KismetArrayLibrary.Array_Add` (`self.GridArray`) _returnvalue_2))))

(fn `UserConstructionScript`)