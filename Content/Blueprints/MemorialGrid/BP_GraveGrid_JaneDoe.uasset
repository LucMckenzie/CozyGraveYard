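; Memorial grid actor (Jane Doe grave variant) that lays out a GridX by GridY field of BP_Tile_GridActor tiles around its location.
; BeginPlay and every Tick check the player character's MemorialCameraActive flag, destroying and respawning the whole grid when true, otherwise hiding the tiles.
; LocationSnapto linearly searches the spawned tiles and returns the location nearest a given point for snapping.
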(event `self.ReceiveTick`
  (params (DeltaSeconds :type "Float (single-precision)"))
  (bind _asbp_test_player_character_2 (cast `/Game/Blueprints/Character/BP_TestPlayerCharacter2` (`GameplayStatics.GetPlayerCharacter` 0) :!label _label))
  (if (`/Game/Blueprints/Character/BP_TestPlayerCharacter2.MemorialCameraActive` _asbp_test_player_character_2)
    (`self.SpawnGrid`)
    (else
      (`self.SetActorHiddenInGame` (`self.Grid Of Actor`) true))))

(event `self.ReceiveBeginPlay`
  (goto _label))

(fn `LocationSnapto`
  (params (In :type "Vector Structure"))
  (returns (Out :type "Vector Structure"))
  (locals (Closest :type "Vector Structure") (Distance :type "Float (double-precision)"))
  (bind _returnvalue (`self.K2_GetActorLocation` (`|GetArrayItem` (`self.Grid Of Actor`))))
  ;[1 1 1] Control Snap to Location
  (set `local.Closest` _returnvalue)
  (set `local.Distance` (`KismetMathLibrary.Vector_Distance` In _returnvalue))
  (for _array_element (`self.Grid Of Actor`)
    (bind _returnvalue_2 (`self.K2_GetActorLocation` _array_element))
    (bind _returnvalue_3 (`KismetMathLibrary.Vector_Distance` _returnvalue_2 In))
    (if (< _returnvalue_3 (`local.Distance`))
      (set `local.Closest` _returnvalue_2)
      (set `local.Distance` _returnvalue_3)))
  (return (`local.Closest`)))

(fn `SpawnGrid`
  (bind (_returnvalue_x _returnvalue_y _returnvalue_z) (`KismetMathLibrary.BreakVector` (`self.K2_GetActorLocation`)))
  (bind _space_between_tiles_ (`self.Space Between Tiles `))
  (bind _grid_y (`self.Grid Y`))
  (bind _grid_x (`self.Grid X`))
  (bind _grid_of_actor (`self.Grid Of Actor`))
  ;[1 1 1] Spawns the Gird
  (for _array_element _grid_of_actor
    (`self.K2_DestroyActor` _array_element))
  (`KismetArrayLibrary.Array_Clear` _grid_of_actor)
  (for _index (range _grid_x)
    (for _index_2 (range _grid_y)
      (bind _returnvalue (`|SpawnActorFromClass` "/Game/Blueprints/MemorialGrid/BP_Tile_GridActor.BP_Tile_GridActor_C" (`KismetMathLibrary.MakeTransform` (`KismetMathLibrary.MakeVector` (+ _returnvalue_x (`KismetMathLibrary.Conv_IntToDouble` (* (- (/ _grid_y 2) _index_2) _space_between_tiles_))) (+ _returnvalue_y (`KismetMathLibrary.Conv_IntToDouble` (* (- (/ _grid_x 2) _index) _space_between_tiles_))) _returnvalue_z)) "Undefined" "OverrideRootScale" null null))
      (`KismetArrayLibrary.Array_Add` (`self.Grid Of Actor`) _returnvalue))))

(fn `UserConstructionScript`)