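; BP_Camera_Activation is an overlap trigger actor that shows the player's grave camera interface on the memorial grid.
; When a BP_TestPlayerCharacter2 holding a memory box enters, it sets ActivateOverlapBoolGraveCamera, adds the character's GraveCameraInterface widget to the viewport and calls CameraActiveSetup.
; When that character leaves, it removes the widget and calls CameraDeactivateSetup, without checking the box or resetting the flag.
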(event `self.ReceiveActorBeginOverlap`
  (params (OtherActor :type "Actor Object Reference"))
  ;[1 1 1] Activate Camera Button
  (bind _asbp_test_player_character_2 (cast `/Game/Blueprints/Character/BP_TestPlayerCharacter2` OtherActor))
  (if (`/Game/Blueprints/Character/BP_TestPlayerCharacter2.IsHoldingMemoryBox` _asbp_test_player_character_2)
    (`KismetSystemLibrary.PrintString` "BoolSet")
    (set `self.ActivateOverlapBool_GraveCamera` true)
    (bind _gravecamerainterface (`/Game/Blueprints/Character/BP_TestPlayerCharacter2.GraveCameraInterface` _asbp_test_player_character_2))
    (`UserWidget.AddToViewport` _gravecamerainterface 0)
    (`/Game/Blueprints/MemorialGrid/W_Memorial_EnterGraveCamera.CameraActive_Setup` _gravecamerainterface "F")))

(event `self.ReceiveActorEndOverlap`
  (params (OtherActor :type "Actor Object Reference"))
  ;[1 1 1] Activate Camera Button
  (bind _asbp_test_player_character_2 (cast `/Game/Blueprints/Character/BP_TestPlayerCharacter2` OtherActor))
  (`KismetSystemLibrary.PrintString` "Remove")
  (bind _gravecamerainterface (`/Game/Blueprints/Character/BP_TestPlayerCharacter2.GraveCameraInterface` _asbp_test_player_character_2))
  (`Widget.RemoveFromParent` _gravecamerainterface)
  (`/Game/Blueprints/MemorialGrid/W_Memorial_EnterGraveCamera.CameraDeactivate_Setup` _gravecamerainterface "None"))

(fn `UserConstructionScript`)