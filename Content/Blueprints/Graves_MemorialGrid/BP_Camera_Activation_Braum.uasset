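; Trigger actor for the Braum grave camera on the memorial grid, offering a camera-activation prompt to the player.
; Each tick, while the player's SetDay2 flag is off, it shows itself and enables the sphere trigger only while the player holds the memory box.
; Overlapping with the box adds the player's GraveCameraInterfaceEnterBraum widget to the viewport; ending overlap or a touch-leave removes it.
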(event `self.ReceiveBeginPlay`
  (`PrimitiveComponent.SetCollisionEnabled` (`self.Sphere Trigger`) "NoCollision")
  (`self.SetActorHiddenInGame` true))

(event `self.ReceiveTick`
  (params (DeltaSeconds :type "Float (single-precision)"))
  (bind _asbp_test_player_character_2 (cast `/Game/Blueprints/Character/BP_TestPlayerCharacter2` (`GameplayStatics.GetPlayerCharacter` 0)))
  (if (`/Game/Blueprints/Character/BP_TestPlayerCharacter2.SetDay2` _asbp_test_player_character_2)
    _
    (elif (`/Game/Blueprints/Character/BP_TestPlayerCharacter2.IsHoldingMemoryBox` _asbp_test_player_character_2)
      (`PrimitiveComponent.SetCollisionEnabled` (`self.Sphere Trigger`) "QueryAndPhysics")
      (`self.SetActorHiddenInGame` false)
      (else
        (`PrimitiveComponent.SetCollisionEnabled` (`self.Sphere Trigger`) "NoCollision")
        (`self.SetActorHiddenInGame` true)))))

(event `self.ReceiveActorBeginOverlap`
  (params (OtherActor :type "Actor Object Reference"))
  ;[1 1 1] Activate Camera Button
  (bind _asbp_test_player_character_2 (cast `/Game/Blueprints/Character/BP_TestPlayerCharacter2` OtherActor))
  (if (`/Game/Blueprints/Character/BP_TestPlayerCharacter2.IsHoldingMemoryBox` _asbp_test_player_character_2)
    (`KismetSystemLibrary.PrintString` "BoolSet")
    (`UserWidget.AddToViewport` (`/Game/Blueprints/Character/BP_TestPlayerCharacter2.GraveCameraInterfaceEnterBraum` _asbp_test_player_character_2) 0)))

(event `self.ReceiveActorEndOverlap`
  (params (OtherActor :type "Actor Object Reference"))
  ;[1 1 1] Activate Camera Button
  (bind _asbp_test_player_character_2 (cast `/Game/Blueprints/Character/BP_TestPlayerCharacter2` OtherActor :!label _label))
  (`KismetSystemLibrary.PrintString` "Remove")
  (`Widget.RemoveFromParent` (`/Game/Blueprints/Character/BP_TestPlayerCharacter2.GraveCameraInterfaceEnterBraum` _asbp_test_player_character_2)))

(event `self.ReceiveActorOnInputTouchLeave`
  (params (FingerIndex :type "ETouchIndex Enum" :default "Touch1"))
  ;[1 1 1] Activate Camera Button
  (goto _label))

(fn `UserConstructionScript`)