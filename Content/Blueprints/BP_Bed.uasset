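; BP_Bed is a bed actor that resets every waterable bush in the level when the player touches it.
; Overlapping its sphere with BP_TestPlayerCharacter2 increments a Touched counter, then fetches all WaterableBush actors.
; Each bush has its Watered value cleared and its berry mesh set to the cyan material.
; An ArrayWaterBush length check is left disconnected and never runs.
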(event `self.Sphere_Col.OnComponentBeginOverlap`
  (params (OverlappedComponent :type "PrimitiveComponent Object Reference") (OtherActor :type "Actor Object Reference") (OtherComp :type "PrimitiveComponent Object Reference") (OtherBodyIndex :type Integer) (bFromSweep :type Boolean) (SweepResult :type "HitResult Structure (by ref)"))
  ;[1 1 1] Touching
  (cast `/Game/Blueprints/Character/BP_TestPlayerCharacter2` OtherActor)
  (`/Engine/EditorBlueprintResources/StandardMacros.IncrementInt` (`self.Touched`)
    (:`  `
      (`|ExecutionSequence`
        (:`then_0`
          (bind _outactors (`GameplayStatics.GetAllActorsOfClass` "/Game/Blueprints/Items/Bush/WaterableBush.WaterableBush_C"))
          (for _array_element _outactors
            (set `/Game/Blueprints/Items/Bush/WaterableBush.Watered` 0 _array_element)
            (`PrimitiveComponent.SetMaterial` (`/Game/Blueprints/Items/Bush/WaterableBush.BushBerries` _array_element) 0 "/Game/Assets/Materials/M_Cyan.M_Cyan")))))))

(fn `UserConstructionScript`)